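; Floating box actor, apparently main-menu decoration, that wanders around its spawn point while its cube tumbles.
; A looping timer regularly rerolls a spin axis, spin speed and target, picking either a point in a box around the spawn or, less often, the Scene component's initial location.
; Tick drives the actor forward while easing its rotation toward the target and spinning the cube.
; MoveTo is empty, and its Timeline lerp is disconnected.
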(event `self.ReceiveBeginPlay`
  (bind _returnvalue (`KismetMathLibrary.RandomPointInBoundingBox` (`self.BirthLocation`) (`KismetMathLibrary.MakeVector` 50.0 50.0 50.0)))
  (set `self.BirthLocation` (`self.K2_GetActorLocation`))
  (set `self.RandomPoint` (`SceneComponent.K2_GetComponentLocation` (`self.Scene`)))
  (`KismetSystemLibrary.K2_SetTimerDelegate` (delegate `CustomEvent_0`) 2.0 true)
  (set `self.RandomVR` (`KismetMathLibrary.RandomUnitVector`) :!label _label)
  (set `self.Speed` (`KismetMathLibrary.RandomFloatInRange` 0.2 2.0))
  (set `self.ToLocation` (select `int` (`KismetMathLibrary.RandomIntegerInRange` 0 3) :`0` _returnvalue :`1` (`self.RandomPoint`) :`2` _returnvalue :`3` _returnvalue))
  (`self.MoveTo`))

(event `CustomEvent_0`
  (goto _label))

(event `self.ReceiveTick`
  (params (DeltaSeconds :type "Float (single-precision)"))
  (bind _speed (`self.Speed`))
  (bind (_randomvr_x _randomvr_y _randomvr_z) (`KismetMathLibrary.BreakVector` (`self.RandomVR`)))
  (`self.K2_AddActorLocalOffset` (`KismetMathLibrary.MakeVector` (* DeltaSeconds 20.0)))
  (`self.K2_SetActorRotation` (`KismetMathLibrary.RInterpTo` (`self.K2_GetActorRotation`) (`KismetMathLibrary.FindLookAtRotation` (`self.K2_GetActorLocation`) (`self.ToLocation`)) (`GameplayStatics.GetWorldDeltaSeconds`) 2.0))
  (`SceneComponent.K2_AddWorldRotation` (`self.Cube`) (`KismetMathLibrary.MakeRotator` (* _speed _randomvr_x) (* _randomvr_y _speed) (* _randomvr_z _speed)) false false))

(event `MoveTo`)

(fn `UserConstructionScript`)