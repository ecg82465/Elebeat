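; Player state for the DJ player, holding profile, selected name and dance-game score, and driving the ranking list.
; BeginPlay builds AnimationList from DT_AnimationMap and, for the local pawn, loads PlayerInfo from the save slot.
; Profile and name RepNotifies raise CheckGate, which Tick holds until the pawn is valid, then calls PlayerInfoUpdate on BP_Player_DJ.
; Score and dance-game RepNotifies refresh the ranking through BP_World_GameMode.
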(event `self.ReceiveBeginPlay`
  (`|ExecutionSequence`
    (:`then_0`
      (bind _outrownames (`DataTableFunctionLibrary.GetDataTableRowNames` "/Game/BluePrint/Model/Animation/DT_AnimationMap.DT_AnimationMap"))
      (for _array_element _outrownames
        (bind _returnvalue (`|GetDataTableRow` "/Game/BluePrint/Model/Animation/DT_AnimationMap.DT_AnimationMap" _array_element)
          (:`then`
            (`BlueprintMapLibrary.Map_Add` (`self.AnimationList`) (`.AnimationName_5_47A1DC9940E034A7631EDEB0CDAE15B5` (break `/Game/BluePrint/Model/Animation/ST_AnimationDate` _returnvalue)) _returnvalue)))))
    (:`then_1`
      (bind _islocal (`/Game/BluePrint/BluePrintFunction/BP_FunctionLibrary.PlayerPawnIsLocal?` (`self.PawnPrivate`)))
      (switch `/Game/BluePrint/BluePrintFunction/EM_PlayerPawnOwner` _islocal
        (:`NewEnumerator1`
          (bind _asbp_elebeat_gi (cast `/Game/BluePrint/AllLevel/BP_Elebeat_GI` (`GameplayStatics.GetGameInstance`)))
          (bind _returnvalue_2 (`GameplayStatics.LoadGameFromSlot` (`/Game/BluePrint/AllLevel/BP_Elebeat_GI.NameSaveSlot` _asbp_elebeat_gi)))
          (bind _asbp_save_game_change (cast `/Game/BluePrint/AllLevel/BP_SaveGame_Change` _returnvalue_2))
          (set `self.PlayerInfo` (`/Game/BluePrint/AllLevel/BP_SaveGame_Change.PlayerInfo` _asbp_save_game_change)))))))

(event `self.ReceiveTick`
  (params (DeltaSeconds :type "Float (single-precision)"))
  (bind _pawnprivate (`self.PawnPrivate`))
  (`|ExecutionSequence`
    (:`then_0`
      (if (`self.CheckGate`)
        (`/Engine/EditorBlueprintResources/StandardMacros.IsValid` _pawnprivate
          (:`Is Valid`
            (bind _asbp_player_dj (cast `/Game/BluePrint/Player/BP_Player_DJ` _pawnprivate)
              (:`then`
                (`/Game/BluePrint/Player/BP_Player_DJ.PlayerInfoUpdate` _asbp_player_dj))
              (:`CastFailed`
                (`KismetSystemLibrary.PrintString` "Cast Failure")))
            (set `self.CheckGate` false)))))))

(event `UpdateRankList`
  (bind _asbp_world_game_mode (cast `/Game/BluePrint/DanceGame/BP_World_GameMode` (`GameplayStatics.GetGameMode`)))
  (`/Game/BluePrint/DanceGame/BP_World_GameMode.UpdateRankingLIst` _asbp_world_game_mode))

(fn `OnRep_PlayerInfo`
  (set `self.CheckGate` true))

(fn `OnRep_PlayerInfo_DanceGame`
  (bind _asbp_world_game_mode (cast `/Game/BluePrint/DanceGame/BP_World_GameMode` (`GameplayStatics.GetGameMode`)))
  (`/Game/BluePrint/DanceGame/BP_World_GameMode.UpdateRankingLIst` _asbp_world_game_mode))

(fn `OnRep_ScoreNum`
  (setmembers `/Game/BluePrint/Model/Dance/ST_DanceGame_PlayerInfo` :`StructRef` (`self.PlayerInfo_DanceGame`) :`Score` (`KismetMathLibrary.FTrunc` (`self.ScoreEnergy `)))
  (`self.UpdateRankList`))

(fn `OnRep_UserSelectName`
  (set `self.CheckGate` true))

(fn `UserConstructionScript`)