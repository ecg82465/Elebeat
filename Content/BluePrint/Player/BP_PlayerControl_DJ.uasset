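; Player controller for the DJ dance game, linking player input to the pawn, HUD, game mode and player state.
; On game-state Begin, the authority starts element spawning through a score calculator component it adds at BeginPlay.
; WASD presses update an input struct, triggering authority-side pawn jumps while the replicated JumpOpen gate is open.
; It also relays score, profile, ranking and box-color updates, toggles a message UI and randomizes dance animations.
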(event `GameTick`
  (params (GameState :type "/Game/BluePrint/Model/Dance/EM_DanceGameState Enum" :default "NewEnumerator0"))
  ;[1 1 1] BeginBattle
  (switch `/Game/BluePrint/Model/Dance/EM_DanceGameState` GameState
    (:`NewEnumerator1`
      (`/Engine/EditorBlueprintResources/ActorMacros.Switch Has Authority`
        (:`Authority`
          (`self.BeginPawnElement`))))
    (:`NewEnumerator4`
      (`self.OpenTIckTokGate` false)
      (`KismetSystemLibrary.PrintString` "EndGame"))))

(event `self.ReceiveBeginPlay`
  ;[1 1 1] Init
  (`|ExecutionSequence`
    (:`then_0`
      (`/Engine/EditorBlueprintResources/ActorMacros.Switch Has Authority`
        (:`Authority`
          (bind _returnvalue (`AddComponent|NODE_AddBP_ScoreCaculater_CMP-0` :`PlayerControl` self))
          (set `self.ScoreCaculater` _returnvalue))))
    (:`then_1`
      (bind _asbp_dance_game_state (cast `/Game/BluePrint/DanceGame/BP_DanceGame_State` (`GameplayStatics.GetGameState`)))
      (add `/Game/BluePrint/DanceGame/BP_DanceGame_State.GameStateTick` _asbp_dance_game_state (delegate `GameTick`)))))

(event `SpawnElement_Local`
  (params (TickTIme :type "Float (double-precision)") (ActiveTime :type "Float (double-precision)"))
  (bind _returnvalue (`self.GetHUD`))
  ;[1 1 1] Init
  (`/Engine/EditorBlueprintResources/StandardMacros.IsValid` _returnvalue
    (:`Is Valid`
      (bind _asbp_player_hud_dance_game (cast `/Game/BluePrint/DanceGame/BP_PlayerHUD_DanceGame` _returnvalue))
      (`/Game/BluePrint/DanceGame/BP_PlayerHUD_DanceGame.SpawnTickToklElement` _asbp_player_hud_dance_game TickTIme ActiveTime))))

(event `OpenTIckTokGate`
  (params (JumpOpen :type Boolean))
  ;[1 1 1] Init
  (set `self.JumpOpen` JumpOpen))

(event `UpdateRankingInfo`
  ;[1 1 1] Score
  (`self.RankingMuticast`))

(event `BeginPawnElement`
  ;[1 1 1] Score
  (`/Game/BluePrint/Player/BP_ScoreCaculater_CMP.BeginSpawnFnc` (`self.ScoreCaculater`) true))

(event `Key|One`
  (params (Key :type "Key Structure"))
  (:`Pressed`
    (bind _asbp_world_game_mode (cast `/Game/BluePrint/DanceGame/BP_World_GameMode` (`GameplayStatics.GetGameMode`)))
    (`/Game/BluePrint/DanceGame/BP_World_GameMode.BeginBattale` _asbp_world_game_mode)))

(event `RankingMuticast`
  ;[1 1 1] Score
  (bind _asbp_player_hud_dance_game (cast `/Game/BluePrint/DanceGame/BP_PlayerHUD_DanceGame` (`self.GetHUD`)))
  (`/Game/BluePrint/DanceGame/BP_PlayerHUD_DanceGame.UpdateRankingLIst` _asbp_player_hud_dance_game))

(event `ChangeBoxColor`
  (params (BoxID :type Integer) (Color :type "Vector Structure"))
  ;[1 1 1] Score
  (`self.UpLoadChangeBoxColor` BoxID Color))

(event `CheckScore`
  (bind (_w_dance _s_dance _a_dance _d_dance) (break `/Game/BluePrint/Model/Dance/ST_DanceGame_PlayerInput_Info` (`self.PlayerInputInfo`)))
  (bind _returnvalue (and (`self.JumpOpen`) (`self.HasAuthority`)))
  ;[1 1 1] Score
  (if _w_dance
    (if _returnvalue
      (bind _asbp_player_dj (cast `/Game/BluePrint/Player/BP_Player_DJ` (`self.K2_GetPawn`)))
      (`/Game/BluePrint/Player/BP_Player_DJ.JumpToLocation_Local` _asbp_player_dj "NewEnumerator2"))
    (elif _s_dance
      (if _returnvalue
        (bind _asbp_player_dj_2 (cast `/Game/BluePrint/Player/BP_Player_DJ` (`self.K2_GetPawn`)))
        (`/Game/BluePrint/Player/BP_Player_DJ.JumpToLocation_Local` _asbp_player_dj_2 "NewEnumerator3"))
      (elif _a_dance
        (if _returnvalue
          (bind _asbp_player_dj_3 (cast `/Game/BluePrint/Player/BP_Player_DJ` (`self.K2_GetPawn`)))
          (`/Game/BluePrint/Player/BP_Player_DJ.JumpToLocation_Local` _asbp_player_dj_3 "NewEnumerator0"))
        (elif _d_dance
          (if _returnvalue
            (bind _asbp_player_dj_4 (cast `/Game/BluePrint/Player/BP_Player_DJ` (`self.K2_GetPawn`)))
            (`/Game/BluePrint/Player/BP_Player_DJ.JumpToLocation_Local` _asbp_player_dj_4 "NewEnumerator1")))))))

(event `UploadUrl`
  (params (InString :type String) (NewParam :type "Actor Object Reference"))
  ;[1 1 1] Upload
  (message `/Game/BluePrint/Interface/I_PlayerInteraction.SetUpString_Setting` NewParam InString))

(event `UpLoadChangeBoxColor`
  (params (BoxId :type Integer) (Color :type "Vector Structure"))
  ;[1 1 1] Score
  (bind _asbp_world_game_mode (cast `/Game/BluePrint/DanceGame/BP_World_GameMode` (`GameplayStatics.GetGameMode`)))
  (`/Game/BluePrint/DanceGame/BP_World_GameMode.ChangeOneBoxColor` _asbp_world_game_mode BoxId Color))

(event `UpLoadPlayerInfo`
  (params (InString :type String) (PlayerImageURL :type String))
  ;[1 1 1] Upload
  (bind _asbp_player_state_dj (cast `/Game/BluePrint/Player/BP_PlayerState_DJ` (`self.PlayerState`)))
  (set `/Game/BluePrint/Player/BP_PlayerState_DJ.PlayerInfo` (make `/Game/BluePrint/Model/ST_PlayerInfo` InString PlayerImageURL) _asbp_player_state_dj))

(event `UploadPlayerAnimationType`
  (params (PlayerAnimationName :type String))
  ;[1 1 1] Upload
  (bind _asbp_player_state_dj (cast `/Game/BluePrint/Player/BP_PlayerState_DJ` (`self.PlayerState`)))
  (set `/Game/BluePrint/Player/BP_PlayerState_DJ.UserAnimationState` (make `/Game/BluePrint/Model/Animation/ST_PlayerAnimation_Type` "NewEnumerator1" PlayerAnimationName) _asbp_player_state_dj))

(event `Key|Enter`
  (params (Key :type "Key Structure"))
  (bind _returnvalue (`GameplayStatics.GetPlayerPawn` 0))
  (bind _returnvalue_2 (`GameplayStatics.GetPlayerController` 0))
  ;[1 1 1] Input
  (:`Pressed`
    (bind _isa (`/Engine/EditorBlueprintResources/StandardMacros.FlipFlop`)
      (:`A`
        (`self.DisableInput` _returnvalue _returnvalue_2)
        (set `self.bShowMouseCursor` _isa))
      (:`B`
        (`self.EnableInput` _returnvalue _returnvalue_2)
        (set `self.bShowMouseCursor` _isa)))
    (`self.ShowEnterUI` self _isa)))

(event `UploadScore`
  (bind _asbp_player_state_dj (cast `/Game/BluePrint/Player/BP_PlayerState_DJ` (`self.PlayerState`) :!pure true))
  ;[1 1 1] Upload
  (set `/Game/BluePrint/Player/BP_PlayerState_DJ.ScoreEnergy ` (+ (`/Game/BluePrint/Player/BP_PlayerState_DJ.ScoreEnergy ` _asbp_player_state_dj) 2.0) _asbp_player_state_dj))

(event `ShowEnterUI`
  (params (InteractionActor :type "Actor Object Reference") (ShowEnter :type Boolean))
  ;[1 1 1] Input
  (message `/Game/BluePrint/Interface/I_PlayerInteraction.OpenEnter` (`self.GetHUD`) InteractionActor ShowEnter))

(event `RemoveElement`
  ;[1 1 1] Upload
  (bind _asbp_player_dj (cast `/Game/BluePrint/Player/BP_Player_DJ` (`self.K2_GetPawn`)))
  (`/Game/BluePrint/Player/BP_Player_DJ.RemoveElement` _asbp_player_dj))

(event `Key|Tab`
  (params (Key :type "Key Structure"))
  ;[1 1 1] Input
  (:`Pressed`
    (`self.SwitchAnimation`)))

(event `InputAction|W_dance` :consume false
  (params (Key :type "Key Structure"))
  ;[1 1 1] Input
  (:`Pressed`
    (`self.UploadInputState` true "W"))
  (:`Released`
    (`self.UploadInputState` false "W")))

(event `InputAction|S_dance` :consume false
  (params (Key :type "Key Structure"))
  ;[1 1 1] Input
  (:`Pressed`
    (`self.UploadInputState` true "S"))
  (:`Released`
    (`self.UploadInputState` false "S")))

(event `SwitchAnimation`
  ;[1 1 1] Caculate  Anim
  (bind _asbp_player_state_dj (cast `/Game/BluePrint/Player/BP_PlayerState_DJ` (`Pawn.PlayerState` (`GameplayStatics.GetPlayerCharacter` 0))))
  (bind _keys (`BlueprintMapLibrary.Map_Keys` (`/Game/BluePrint/Player/BP_PlayerState_DJ.AnimationList` _asbp_player_state_dj) :!label _label))
  (set `self.Now_AnimationIndex` (`KismetMathLibrary.RandomInteger` (`KismetArrayLibrary.Array_Length` _keys)))
  (bind _output (`|GetArrayItem` _keys (`self.Now_AnimationIndex`)))
  (if (`KismetStringLibrary.EqualEqual_StrStr` (`.AnimationName_4_06351A0344C5C4E489BA7F8DE20E1916` (break `/Game/BluePrint/Model/Animation/ST_PlayerAnimation_Type` (`/Game/BluePrint/Player/BP_PlayerState_DJ.UserAnimationState` _asbp_player_state_dj))) _output)
    (goto _label)
    (else
      (`self.UploadPlayerAnimationType` _output))))

(event `InputAction|A_dance` :consume false
  (params (Key :type "Key Structure"))
  ;[1 1 1] Input
  (:`Pressed`
    (`self.UploadInputState` true "A"))
  (:`Released`
    (`self.UploadInputState` false "A")))

(event `UploadInputState`
  (params (Pressed :type Boolean) (InputName :type String))
  (bind _playerinputinfo (`self.PlayerInputInfo`))
  ;[1 1 1] Input
  (switch `string` InputName
    (:`W`
      (setmembers `/Game/BluePrint/Model/Dance/ST_DanceGame_PlayerInput_Info` :`StructRef` _playerinputinfo :`W_Dance` Pressed))
    (:`S`
      (setmembers `/Game/BluePrint/Model/Dance/ST_DanceGame_PlayerInput_Info` :`StructRef` _playerinputinfo :`S_Dance` Pressed))
    (:`A`
      (setmembers `/Game/BluePrint/Model/Dance/ST_DanceGame_PlayerInput_Info` :`StructRef` _playerinputinfo :`A_Dance` Pressed))
    (:`D`
      (setmembers `/Game/BluePrint/Model/Dance/ST_DanceGame_PlayerInput_Info` :`StructRef` _playerinputinfo :`D_Dance` Pressed))
    (:`TAB`
      (setmembers `/Game/BluePrint/Model/Dance/ST_DanceGame_PlayerInput_Info` :`StructRef` _playerinputinfo :`Tab` Pressed)))
  (`self.CheckScore`))

(event `InputAction|D_dance` :consume false
  (params (Key :type "Key Structure"))
  ;[1 1 1] Input
  (:`Pressed`
    (`self.UploadInputState` true "D"))
  (:`Released`
    (`self.UploadInputState` false "D")))

(event `InputAction|TAB_dance`
  (params (Key :type "Key Structure"))
  ;[1 1 1] Input
  (:`Pressed`
    (`self.UploadInputState` true "TAB"))
  (:`Released`
    (`self.UploadInputState` false "TAB")))

(fn `OnRep_JumpOpen`)

(fn `SetUpPlayerInfo`
  (params (PlayerID :type Integer))
  (`|ExecutionSequence`
    (:`then_0`
      (bind _asbp_elebeat_gi (cast `/Game/BluePrint/AllLevel/BP_Elebeat_GI` (`GameplayStatics.GetGameInstance`)))
      (bind _returnvalue (`GameplayStatics.LoadGameFromSlot` (`/Game/BluePrint/AllLevel/BP_Elebeat_GI.NameSaveSlot` _asbp_elebeat_gi)))
      (bind _asbp_save_game_change (cast `/Game/BluePrint/AllLevel/BP_SaveGame_Change` _returnvalue))
      (bind _asbp_player_state_dj (cast `/Game/BluePrint/Player/BP_PlayerState_DJ` (`self.PlayerState`)))
      (set `/Game/BluePrint/Player/BP_PlayerState_DJ.PlayerInfo` (`/Game/BluePrint/AllLevel/BP_SaveGame_Change.PlayerInfo` _asbp_save_game_change) _asbp_player_state_dj))
    (:`then_1`
      (set `self.PlayerID` PlayerID))))

(fn `UserConstructionScript`)