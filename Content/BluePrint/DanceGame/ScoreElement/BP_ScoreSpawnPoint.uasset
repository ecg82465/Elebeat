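; BP_ScoreSpawnPoint is the dance game's anchor actor that spawns and holds score elements around a player.
; Each tick it snaps to the player mesh set through Init and smoothly turns its yaw along the camera-to-actor direction.
; SpawnMuticast creates a BP_ScoreElement from a message, offset from the Begin component, then attaches and queues it.
; RemoveElement dismisses the oldest queued element first.
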(event `SpawnMuticast`
  (params (Message :type "/Game/BluePrint/Model/Dance/Score/ST_ElementMessage Structure"))
  (bind _returnvalue (`|SpawnActorFromClass` "/Game/BluePrint/DanceGame/ScoreElement/BP_ScoreElement.BP_ScoreElement_C" (`KismetMathLibrary.MakeTransform` (+ (`.RelativeLocation_10_92E65BB34BF39850C2356D95A46D8096` (break `/Game/BluePrint/Model/Dance/Score/ST_ElementMessage` Message)) (`SceneComponent.K2_GetComponentLocation` (`self.Begin`)))) "Undefined" "OverrideRootScale" null Message null))
  (`KismetArrayLibrary.Array_Add` (`self.Element_List_Ref`) _returnvalue)
  (`self.K2_AttachToActor` _returnvalue self "None" "KeepWorld" "KeepWorld" "KeepWorld" true))

(event `self.ReceiveTick`
  (params (DeltaSeconds :type "Float (single-precision)"))
  (`|ExecutionSequence`
    (:`then_0`
      (`self.FaceToCamera`))))

(event `RemoveElement`
  (bind _element_list_ref (`self.Element_List_Ref`))
  (bind _output (`|GetArrayItem` _element_list_ref))
  (`/Engine/EditorBlueprintResources/StandardMacros.IsValid` _output
    (:`Is Valid`
      (`/Game/BluePrint/DanceGame/ScoreElement/BP_ScoreElement.RemoveMe` _output)
      (`KismetArrayLibrary.Array_Remove` _element_list_ref))))

(fn `FaceToCamera`
  (bind _playerpawn (`self.PlayerPawn`))
  (bind (_returnvalue_roll _returnvalue_pitch _returnvalue_yaw) (`KismetMathLibrary.BreakRotator` (`KismetMathLibrary.FindLookAtRotation` (`SceneComponent.K2_GetComponentLocation` (`/Game/BluePrint/Player/BP_Player_DJ.Camera` _playerpawn)) (`self.K2_GetActorLocation`))))
  (`/Engine/EditorBlueprintResources/StandardMacros.IsValid` _playerpawn
    (:`Is Valid`
      (`self.K2_SetActorLocationAndRotation` (`SceneComponent.K2_GetComponentLocation` (`Character.Mesh` _playerpawn)) (`KismetMathLibrary.RInterpTo` (`self.K2_GetActorRotation`) (`KismetMathLibrary.MakeRotator` 0.0 0.0 _returnvalue_yaw) (`GameplayStatics.GetWorldDeltaSeconds`) 2.0)))))

(fn `Init`
  (params (PlayerPawn :type "/Game/BluePrint/Player/BP_Player_DJ Object Reference"))
  (set `self.PlayerPawn` PlayerPawn))

(fn `UserConstructionScript`)