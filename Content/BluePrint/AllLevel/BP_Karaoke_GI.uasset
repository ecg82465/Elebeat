(event `SaveGameCheck`
  (bind _returnvalue (`GameplayStatics.DoesSaveGameExist` (`self.NameSaveSlot`)))
  (if _returnvalue
    (`self.ShowMainMenu`)
    (else
      (`self.ShowPlayerSetting`)
      (set `PlayerController.bShowMouseCursor` true (`GameplayStatics.GetPlayerController` 0)))))

(event `ShowMainMenu`
  ;[1 1 1] 显示主菜单
  (`/Engine/EditorBlueprintResources/StandardMacros.IsValid` (`self.MainMenu`)
    (:`Is Valid`
      _)
    (:`Is Not Valid`
      (bind _returnvalue (`|CreateWidget` "/Game/BluePrint/UMG/MainMenu/MainMenuUmg.MainMenuUmg_C" (`GameplayStatics.GetPlayerController` 0)))
      (set `self.MainMenu` _returnvalue)))
  (`UserWidget.AddToViewport` (`self.MainMenu`) 0)
  (set `PlayerController.bShowMouseCursor` true (`GameplayStatics.GetPlayerController` 0)))

(event `ShowLoadingScreen`
  (bind _returnvalue (`|CreateWidget` "/Game/BluePrint/UMG/AllLevel/LoadingScreen.LoadingScreen_C" (`GameplayStatics.GetPlayerController` 0)))
  (`UserWidget.AddToViewport` _returnvalue 0))

(event `ShowRoomSetting`
  ;[1 1 1] 显示房间设置
  (`/Engine/EditorBlueprintResources/StandardMacros.IsValid` (`self.RoomSetting`)
    (:`Is Valid`
      _)
    (:`Is Not Valid`
      (bind _returnvalue (`|CreateWidget` "/Game/BluePrint/UMG/MainMenu/RoomSetting.RoomSetting_C" (`GameplayStatics.GetPlayerController` 0)))
      (set `self.RoomSetting` _returnvalue)))
  (`UserWidget.AddToViewport` (`self.RoomSetting`) 0))

(event `CreateRoom`
  (params (`Lan?` :type Boolean) (ServerName :type String) (MaxPlayer :type Integer))
  (bind _output_get (set `self.MaxPlayer` MaxPlayer))
  (set `self.ServerName` ServerName)
  (`self.ShowLoadingScreen`)
  (`CreateSessionCallbackProxy.CreateSession` (`GameplayStatics.GetPlayerController` 0) _output_get `Lan?`
    (:`OnSuccess`
      (`GameplayStatics.OpenLevel` "World_Test01" true "listen"))
    (:`OnFailure`
      (`KismetSystemLibrary.PrintString` "fail"))))

(event `JoinServer`
  (params (SearchResult :type "BlueprintSessionResult Structure (by ref)"))
  (`self.ShowLoadingScreen`)
  (`JoinSessionCallbackProxy.JoinSession` (`GameplayStatics.GetPlayerController` 0) SearchResult))

(event `ShowServerMenu`
  ;[1 1 1] 显示搜索菜单
  (`/Engine/EditorBlueprintResources/StandardMacros.IsValid` (`self.ServerMenu`)
    (:`Is Valid`
      _)
    (:`Is Not Valid`
      (bind _returnvalue (`|CreateWidget` "/Game/BluePrint/UMG/MainMenu/FindMenu.FindMenu_C" (`GameplayStatics.GetPlayerController` 0)))
      (set `self.ServerMenu` _returnvalue)))
  (`UserWidget.AddToViewport` (`self.ServerMenu`) 0))

(event `ShowPlayerSetting`
  ;[1 1 1] 显示玩家设置界面
  (`/Engine/EditorBlueprintResources/StandardMacros.IsValid` (`self.PlayerSetting`)
    (:`Is Valid`
      _)
    (:`Is Not Valid`
      (bind _returnvalue (`|CreateWidget` "/Game/BluePrint/UMG/MainMenu/PlayerSetting.PlayerSetting_C" (`GameplayStatics.GetPlayerController` 0)))
      (set `self.PlayerSetting` _returnvalue)))
  (`UserWidget.AddToViewport` (`self.PlayerSetting`) 0))

(event `ShowRoomList`
  ;[1 1 1] 显示房间列表
  (`/Engine/EditorBlueprintResources/StandardMacros.IsValid` (`self.RoomList`)
    (:`Is Valid`
      _)
    (:`Is Not Valid`
      (bind _returnvalue (`|CreateWidget` "/Game/BluePrint/UMG/MainMenu/RoomList/U_RoomList.U_RoomList_C" (`GameplayStatics.GetPlayerController` 0)))
      (set `self.RoomList` _returnvalue)))
  (`UserWidget.AddToViewport` (`self.RoomList`) 0))