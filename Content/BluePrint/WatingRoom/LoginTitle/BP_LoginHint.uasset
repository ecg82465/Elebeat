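; BP_LoginHint is a login title hint in the waiting room that animates a Cylinder's material, apparently as a progress indicator.
; ToLocation sets a target and opens an animation gate, and Tick then raises Num at a constant rate, writing it to the material's "Num" scalar until it reaches that target.
; Pressing the 3 key steps the target up, which looks like a test trigger.
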(event `Key|Three`
  (params (Key :type "Key Structure"))
  (:`Pressed`
    (bind _output_get (set `self.NewVar_0` (+ (`self.NewVar_0`) 0.1)))
    (`self.ToLocation` _output_get)))

(event `ToLocation`
  (params (NewParam :type "Float (double-precision)"))
  (set `self.ToNum` NewParam)
  (set `self.InAnimationGate` true))

(event `self.ReceiveTick`
  (params (DeltaSeconds :type "Float (single-precision)"))
  (if (`self.InAnimationGate`)
    (bind _output_get (set `self.Num` (+ (`self.Num`) (* (`GameplayStatics.GetWorldDeltaSeconds`) 0.5))))
    (if (>= _output_get (`self.ToNum`))
      (set `self.InAnimationGate` false)
      (else
        (`MeshComponent.SetScalarParameterValueOnMaterials` (`self.Cylinder`) "Num" _output_get)))))

(fn `UserConstructionScript`)