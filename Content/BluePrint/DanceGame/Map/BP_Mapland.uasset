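; BP_Mapland builds an animated floor of static mesh tiles laid out in concentric square rings for the DanceGame map.
; The construction script walks each ring's sides through GluttonousSnake, which places tiles along a direction from a moving head point.
; Each tile gets a dynamic material with a numeric "Num" parameter and joins ListMesh.
; Tick offsets each tile's height by a sine of time and list index, sending a wave along the path.
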(event `self.ReceiveTick`
  (params (DeltaSeconds :type "Float (single-precision)"))
  (set `self.Time` (+ (`self.Time`) DeltaSeconds))
  (for (_array_element _array_index) (`self.List_Mesh`)
    (bind (_relativelocation_x _relativelocation_y) (`KismetMathLibrary.BreakVector` (`SceneComponent.RelativeLocation` _array_element)))
    (`SceneComponent.K2_SetRelativeLocation` _array_element (`KismetMathLibrary.MakeVector` _relativelocation_x _relativelocation_y (* (`KismetMathLibrary.Sin` (+ (/ (`KismetMathLibrary.Conv_IntToDouble` _array_index) 2.0) (`self.Time`))) 33.0)) false false)))

(event `Key|Two`
  (params (Key :type "Key Structure")))

(fn `GluttonousSnake`
  (params (LastIndex :type Integer) (A :type "Vector Structure"))
  (returns (NewParam :type Boolean))
  (for _index (range (+ LastIndex 1))
    (bind _result (`/Engine/EditorBlueprintResources/StandardMacros.IncrementInt` (`self.Index`))
      (:`  `
        (bind _returnvalue (+ (`self.TempHead`) (* A (* (`KismetMathLibrary.Conv_IntToDouble` _index) (`self.Range`)))))
        (bind _returnvalue_2 (`AddComponent|NODE_AddStaticMeshComponent-1` :`RelativeTransform` (`KismetMathLibrary.MakeTransform` _returnvalue (struct) (5.0 5.0 5.0))))
        (bind _returnvalue_3 (`PrimitiveComponent.CreateDynamicMaterialInstance` _returnvalue_2 0 "/Engine/BasicShapes/BasicShapeMaterial.BasicShapeMaterial" "None"))
        (`MaterialInstanceDynamic.SetScalarParameterValue` _returnvalue_3 "Num" (`KismetMathLibrary.Conv_IntToDouble` _result))
        (`KismetArrayLibrary.Array_Add` (`self.List_Mesh`) _returnvalue_2))))
  (set `self.TempHead` _returnvalue)
  (return false))

(fn `UserConstructionScript`
  (`KismetArrayLibrary.Array_Clear` (`self.List_Mesh`))
  (for _index (range (`self.Circle`))
    (bind _returnvalue (* (* _index (`self.Range`)) -1.0))
    (set `self.TempHead` (`KismetMathLibrary.MakeVector` _returnvalue _returnvalue))
    (if (== _index 0)
      (`self.GluttonousSnake` 0 (0.0 1.0 0.0))
      (`self.GluttonousSnake` 0 (-1.0 0.0 0.0))
      (`self.GluttonousSnake` 1 (0.0 -1.0 0.0))
      (else
        (bind _returnvalue_2 (* _index 2))
        (`self.GluttonousSnake` (- _returnvalue_2 1) (1.0 0.0 0.0))
        (`self.GluttonousSnake` _returnvalue_2 (0.0 1.0 0.0))
        (`self.GluttonousSnake` _returnvalue_2 (-1.0 0.0 0.0))
        (`self.GluttonousSnake` (+ _returnvalue_2 1) (0.0 -1.0 0.0))))))