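; A single box tile of the dance game map that serves as a jump target for BP_Player_DJ.
; Down and Up events matching its circle index lower or restore it via timeline, while PlayAnim bobs the mesh on a sine wave phased by tile number and BPMapLand time.
; Trigger returns the jump location within range, otherwise resets colour and hides the direction indicator, which setup events show snapped to 90-degree yaw steps.
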(event `self.ReceiveBeginPlay`
  (set `self.BrithLocation` (`self.K2_GetActorLocation`)))

(event `Down`
  (params (NewParam :type Integer))
  (if (== (`self.MyCircle`) NewParam)
    (set `self.CurrentHight` -300.0)
    (bind (_direction _newtrack_0) (`Timeline|EE` :!label _label)
      (:`Update`
        (`self.K2_SetActorLocation` (+ (`self.BrithLocation`) (`KismetMathLibrary.MakeVector` 0.0 0.0 (`KismetMathLibrary.Lerp` 0.0 -300.0 _newtrack_0))))))))

(event `Up`
  (params (B :type Integer))
  (if (== (`self.MyCircle`) B)
    (set `self.CurrentHight` 0.0)
    (goto _label :!via `Reverse`)))

(event `PlayAnim`
  (bind _sm_box (`self.SM_Box`))
  (bind (_relativelocation_x _relativelocation_y _relativelocation_z) (`KismetMathLibrary.BreakVector` (`SceneComponent.RelativeLocation` _sm_box)))
  (`Timeline|Timeline_0` :!via `PlayFromStart`
    (:`Update`
      (`SceneComponent.K2_SetRelativeLocation` _sm_box (`KismetMathLibrary.MakeVector` _relativelocation_x _relativelocation_y (`KismetMathLibrary.FInterpTo` _relativelocation_z (* (`KismetMathLibrary.Sin` (+ (/ (`KismetMathLibrary.Conv_IntToDouble` (`self.MyNum`)) 2.0) (`/Game/BluePrint/DanceGame/BOXMap/BP_Mapland.Time` (`self.BP_MapLand`)))) 33.0) (`GameplayStatics.GetWorldDeltaSeconds`) 2.0)) false false))))

(event `/Game/BluePrint/Interface/I_PlayerInteraction.SetUpVectir_Setting`
  (params (Color :type "Vector Structure"))
  (`PrimitiveComponent.SetMaterial` (`self.SM_Box`) 0 "/Game/Mateirals/Red_color.Red_color"))

(event `/Game/BluePrint/Interface/I_PlayerInteraction.SetUpString_Setting`
  (params (String :type String))
  (bind _ui_diraction (`self.UI_Diraction`))
  (bind (_returnvalue_roll _returnvalue_pitch _returnvalue_yaw) (`KismetMathLibrary.BreakRotator` (`KismetMathLibrary.FindLookAtRotation` (`self.K2_GetActorLocation` (`GameplayStatics.GetPlayerPawn` 0)) (`SceneComponent.K2_GetComponentLocation` (`self.BodyLocation`)))))
  (switch `string` String
    (:`Left`
      (`SceneComponent.SetHiddenInGame` _ui_diraction false false)
      (`SceneComponent.K2_SetRelativeRotation` _ui_diraction (`KismetMathLibrary.MakeRotator` 0.0 0.0 (* (`KismetMathLibrary.FFloor` (/ (+ _returnvalue_yaw 90.0) 90.0)) 90.0)) false false :!label _label_2))
    (:`Right`
      (`SceneComponent.SetHiddenInGame` _ui_diraction false false)
      (goto _label_2))
    (:`Front`
      (`SceneComponent.SetHiddenInGame` _ui_diraction false false)
      (goto _label_2))
    (:`Back`
      (`SceneComponent.SetHiddenInGame` _ui_diraction false false)
      (goto _label_2))
    (:`Hidding`
      (`SceneComponent.SetHiddenInGame` _ui_diraction true false))))

(fn `GetJumpLocation`
  (returns (ReturnValue :type "Vector Structure"))
  (return (`SceneComponent.K2_GetComponentLocation` (`self.BodyLocation`))))

(fn `Trigger `
  (params (`Begin?` :type Boolean) (TriggerActor :type "Actor Object Reference"))
  (returns (Location :type "Vector Structure"))
  (locals (NewLocalVar_0 :type "Vector Structure"))
  (bind _returnvalue (`KismetMathLibrary.VSize` (- (`SceneComponent.K2_GetComponentLocation` (`self.TargetPoint`)) (`self.K2_GetActorLocation` TriggerActor))))
  (bind _asbp_player_dj (cast `/Game/BluePrint/Player/BP_Player_DJ` TriggerActor))
  (if (and `Begin?` (and (>= _returnvalue 100.0) (<= _returnvalue (`self.JumRange`))))
    (return (`SceneComponent.K2_GetComponentLocation` (`self.BodyLocation`)))
    (else
      (`MeshComponent.SetVectorParameterValueOnMaterials` (`self.SM_Box`) "Color" (1.0 1.0 1.0))
      (`SceneComponent.SetHiddenInGame` (`self.UI_Diraction`) true false)
      (return (0.0 0.0 0.0)))))

(fn `UserConstructionScript`)