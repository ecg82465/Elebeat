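; Game mode for a multiplayer dance battle that manages players, music selection, match timing and rankings.
; It loads songs from a music data table and, on each login, refreshes every player's setup with zero score and random color.
; Battle start picks a random song; Tick then updates game time through a delay and switches state at the limit.
; Rankings sort player info by ascending score into the game state, and box color changes forward to the board.
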(event `self.ReceiveBeginPlay`
  (bind _outrownames (`DataTableFunctionLibrary.GetDataTableRowNames` "/Game/BluePrint/Model/Music/DT_MusicMap.DT_MusicMap"))
  (for _array_element _outrownames
    (bind _returnvalue (`|GetDataTableRow` "/Game/BluePrint/Model/Music/DT_MusicMap.DT_MusicMap" _array_element)
      (:`then`
        (`KismetArrayLibrary.Array_Add` (`self.SoundList`) _returnvalue)))))

(event `self.K2_PostLogin`
  (params (NewPlayer :type "PlayerController Object Reference"))
  (bind _allplayerlist (`self.AllPlayerList`))
  (`KismetArrayLibrary.Array_Add` _allplayerlist NewPlayer)
  (for (_array_element _array_index) _allplayerlist
    (bind _asbp_player_control_dj (cast `/Game/BluePrint/Player/BP_PlayerControl_DJ` _array_element))
    (`/Game/BluePrint/Player/BP_PlayerControl_DJ.SetUpPlayerInfo` _asbp_player_control_dj _array_index)
    (bind _asbp_player_state_dj (cast `/Game/BluePrint/Player/BP_PlayerState_DJ` (`Controller.PlayerState` _asbp_player_control_dj)))
    (set `/Game/BluePrint/Player/BP_PlayerState_DJ.PlayerInfo_DanceGame` (make `/Game/BluePrint/Model/Dance/ST_DanceGame_PlayerInfo` (`.PlayerName_5_F00CFD8D4C06B9002302EC9E45644B27` (break `/Game/BluePrint/Model/ST_PlayerInfo` (`/Game/BluePrint/Player/BP_PlayerState_DJ.PlayerInfo` _asbp_player_state_dj))) 0 (`KismetMathLibrary.RandomUnitVector`)) _asbp_player_state_dj)))

(event `BeginBattale`
  (bind _soundlist (`self.SoundList`))
  (bind _asbp_dance_game_state (cast `/Game/BluePrint/DanceGame/BP_DanceGame_State` (`GameplayStatics.GetGameState`)))
  (if (not (`/Game/BluePrint/DanceGame/BP_DanceGame_State.BattleBegin` _asbp_dance_game_state))
    (set `/Game/BluePrint/DanceGame/BP_DanceGame_State.BattleBegin` true _asbp_dance_game_state)
    (set `/Game/BluePrint/DanceGame/BP_DanceGame_State.NowBackGroundMusic` (`|GetArrayItem` _soundlist (`KismetMathLibrary.RandomIntegerInRange` 0 (- (`KismetArrayLibrary.Array_Length` _soundlist) 1))) _asbp_dance_game_state)
    (`/Game/BluePrint/DanceGame/BP_DanceGame_State.ChangeGameState_Server` _asbp_dance_game_state "NewEnumerator0")
    (`self.UpdateRankingLIst`)))

(event `self.ReceiveTick`
  (params (DeltaSeconds :type "Float (single-precision)"))
  (bind _asbp_dance_game_state (cast `/Game/BluePrint/DanceGame/BP_DanceGame_State` (`GameplayStatics.GetGameState`) :!pure true))
  ;[1 1 1] Time
  (if (`/Game/BluePrint/DanceGame/BP_DanceGame_State.BattleBegin` (cast `/Game/BluePrint/DanceGame/BP_DanceGame_State` (`GameplayStatics.GetGameState`) :!pure true))
    (bind _output_get (set `self.GameTime` (+ DeltaSeconds (`self.GameTime`))))
    (`|ExecutionSequence`
      (:`then_0`
        (if (>= _output_get (`/Game/BluePrint/DanceGame/BP_DanceGame_State.Max_GameTime` _asbp_dance_game_state))
          (`/Game/BluePrint/DanceGame/BP_DanceGame_State.ChangeGameState_Server` _asbp_dance_game_state "NewEnumerator4")))
      (:`then_1`
        (`KismetSystemLibrary.Delay` 1.0)
        (`/Game/BluePrint/DanceGame/BP_DanceGame_State.SetUpGameInfo` _asbp_dance_game_state (`self.GameTime`))))))

(event `UpdateRankingLIst`
  (bind _rankinglist (`self.RankingList`))
  ;[1 1 1] Sort RankLIst
  (`KismetSystemLibrary.PrintString` "GameMode: RefrashRank_List" true true (struct :`R` 1.0 :`G` 0.868115 :`A` 1.0))
  (`KismetArrayLibrary.Array_Clear` (`self.RankingList`))
  (for _array_element (`self.AllPlayerList`)
    (bind _asbp_player_state_dj (cast `/Game/BluePrint/Player/BP_PlayerState_DJ` (`Controller.PlayerState` _array_element)))
    (`KismetArrayLibrary.Array_Add` _rankinglist (`/Game/BluePrint/Player/BP_PlayerState_DJ.PlayerInfo_DanceGame` _asbp_player_state_dj)))
  (bind _st_dancegame_playerinfo (`self.SortScroceList` _rankinglist))
  (bind _asbp_dance_game_state (cast `/Game/BluePrint/DanceGame/BP_DanceGame_State` (`GameplayStatics.GetGameState`)))
  (set `/Game/BluePrint/DanceGame/BP_DanceGame_State.Rank_PlayerList` _st_dancegame_playerinfo _asbp_dance_game_state))

(event `ChangeOneBoxColor`
  (params (BoxID :type Integer) (NewParam2 :type "Vector Structure"))
  (`/Game/BluePrint/DanceGame/BOXMap/BP_Mapland.ChangeBoxColor_Server` (`self.GamePlay_BoxLand`) BoxID NewParam2))

(fn `SortScroceList`
  (params (ST_DanceGame_PlayerInfo1 :type "Array of /Game/BluePrint/Model/Dance/ST_DanceGame_PlayerInfo Structure (by ref)"))
  (returns (ST_DanceGame_PlayerInfo :type "Array of /Game/BluePrint/Model/Dance/ST_DanceGame_PlayerInfo Structure"))
  (locals (LocalRank :type "Array of /Game/BluePrint/Model/Dance/ST_DanceGame_PlayerInfo Structure") (LocalScoreNumber :type "Array of Integer") (CurrentMin :type Integer) (OutRank :type "Array of /Game/BluePrint/Model/Dance/ST_DanceGame_PlayerInfo Structure"))
  (bind _localscorenumber (`local.LocalScoreNumber`))
  (bind _output_get (set `local.LocalRank` ST_DanceGame_PlayerInfo1))
  (for _array_element _output_get
    (`KismetArrayLibrary.Array_Add` (`local.LocalScoreNumber`) (`.Score_5_66CC3BE14122ADFC623416BC0A86FEE1` (break `/Game/BluePrint/Model/Dance/ST_DanceGame_PlayerInfo` _array_element))))
  (while (> (`KismetArrayLibrary.Array_Length` _localscorenumber) 0)
    (bind _output_get_2 (set `local.CurrentMin` (`KismetMathLibrary.MinOfIntArray` _localscorenumber)))
    (`KismetArrayLibrary.Array_Add` (`local.OutRank`) (`|GetArrayItem` (`local.LocalRank`) _output_get_2))
    (`KismetArrayLibrary.Array_Remove` _localscorenumber _output_get_2)
    (`KismetArrayLibrary.Array_Remove` (`local.LocalRank`) _output_get_2))
  (return (`local.OutRank`)))

(fn `UserConstructionScript`)