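; HUD for the dance game that creates and drives the player's on-screen widgets.
; On BeginPlay it adds the main player HUD and binds to the DJ player controller's game-state update, showing a battle-begin widget on Ready.
; It forwards ranking-list and tick-tock element requests to the main HUD.
; OpenEnter lazily creates, shows or removes an enter prompt, passing it the interaction actor.
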(event `CreateBeginUI`
  (params (Action :type "/Game/BluePrint/Model/Dance/EM_DanceGameState Enum" :default "NewEnumerator0"))
  (switch `/Game/BluePrint/Model/Dance/EM_DanceGameState` Action
    (:`NewEnumerator0`
      (bind _returnvalue (`|CreateWidget` "/Game/BluePrint/UMG/DanceGame/BeginPlay/U_BattleBegin.U_BattleBegin_C"))
      (`UserWidget.AddToViewport` _returnvalue 0))))

(event `self.ReceiveBeginPlay`
  (bind _returnvalue (`|CreateWidget` "/Game/BluePrint/UMG/DanceGame/U_PLayerHUD.U_PLayerHUD_C"))
  (set `self.PlayerHUD` _returnvalue)
  (`UserWidget.AddToViewport` _returnvalue 0)
  (bind _asbp_player_control_dj (cast `/Game/BluePrint/Player/BP_PlayerControl_DJ` (`self.GetOwningPlayerController`)))
  (add `/Game/BluePrint/Player/BP_PlayerControl_DJ.UpdateDanceGameState` _asbp_player_control_dj (delegate `CreateBeginUI`)))

(event `/Game/BluePrint/Interface/I_PlayerInteraction.OpenEnter`
  (params (ReturnActor :type "Actor Object Reference") (ShowEnter :type Boolean))
  (bind _playerenter (`self.PlayerEnter`))
  (bind _playerenter_2 (`self.PlayerEnter`))
  (bind _interactionactor (`self.InteractionActor`))
  (set `self.InteractionActor` ReturnActor)
  (if ShowEnter
    (`/Engine/EditorBlueprintResources/StandardMacros.IsValid` (`self.PlayerEnter`)
      (:`Is Valid`
        _)
      (:`Is Not Valid`
        (bind _returnvalue (`|CreateWidget` "/Game/BluePrint/UMG/DanceGame/Interaction/U_PlayerEnter.U_PlayerEnter_C" (`GameplayStatics.GetPlayerController` 0)))
        (set `self.PlayerEnter` _returnvalue)))
    (if (not (`Widget.IsVisible` _playerenter))
      (`UserWidget.AddToViewport` _playerenter 0))
    (`/Engine/EditorBlueprintResources/StandardMacros.IsValid` _interactionactor
      (:`Is Valid`
        (`/Game/BluePrint/UMG/DanceGame/Interaction/U_PlayerEnter.GetReturnObject` _playerenter _interactionactor)))
    (else
      (`/Engine/EditorBlueprintResources/StandardMacros.IsValid` _playerenter_2
        (:`Is Valid`
          (`Widget.RemoveFromParent` _playerenter_2))))))

(event `UpdateRankingLIst`
  (`/Game/BluePrint/UMG/DanceGame/U_PLayerHUD.UpdateRankingList` (`self.PlayerHUD`)))

(event `SpawnTickToklElement`
  (params (TickTIme :type "Float (double-precision)") (ActiveTime :type "Float (double-precision)"))
  (`/Game/BluePrint/UMG/DanceGame/U_PLayerHUD.SpawnTickTokElement` (`self.PlayerHUD`) TickTIme ActiveTime))

(fn `Trigger `
  (params (`Begin?` :type Boolean) (TriggerActor :type "Actor Object Reference"))
  (returns (Location :type "Vector Structure"))
  (return (0.0 0.0 0.0)))

(fn `UserConstructionScript`)