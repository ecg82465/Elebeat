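; Waiting room HUD that shows and hides a player enter widget tied to an interaction actor.
; The OpenEnter event stores the passed actor, then lazily creates and caches U_PlayerEnter for player 0, adds it to the viewport and hands it that actor.
; When the show flag is false, it removes the widget from its parent but keeps the reference for reuse.
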(event `/Game/BluePrint/Interface/I_PlayerInteraction.OpenEnter`
  (params (ReturnActor :type "Actor Object Reference") (ShowEnter :type Boolean))
  (bind _playerenter (`self.PlayerEnter`))
  (bind _playerenter_2 (`self.PlayerEnter`))
  (bind _interactionactor (`self.InteractionActor`))
  (set `self.InteractionActor` ReturnActor)
  (if ShowEnter
    (`/Engine/EditorBlueprintResources/StandardMacros.IsValid` (`self.PlayerEnter`)
      (:`Is Valid`
        _)
      (:`Is Not Valid`
        (bind _returnvalue (`|CreateWidget` "/Game/BluePrint/UMG/DanceGame/Interaction/U_PlayerEnter.U_PlayerEnter_C" (`GameplayStatics.GetPlayerController` 0)))
        (set `self.PlayerEnter` _returnvalue)))
    (if (not (`Widget.IsVisible` _playerenter))
      (`UserWidget.AddToViewport` _playerenter 0))
    (`/Engine/EditorBlueprintResources/StandardMacros.IsValid` _interactionactor
      (:`Is Valid`
        (`/Game/BluePrint/UMG/DanceGame/Interaction/U_PlayerEnter.GetReturnObject` _playerenter _interactionactor)))
    (else
      (`/Engine/EditorBlueprintResources/StandardMacros.IsValid` _playerenter_2
        (:`Is Valid`
          (`Widget.RemoveFromParent` _playerenter_2))))))

(fn `UserConstructionScript`)