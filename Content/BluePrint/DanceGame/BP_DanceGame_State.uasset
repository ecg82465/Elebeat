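; Game state Blueprint for the dance game, driving match phases and holding game time, background music and ranking data.
; A server event multicasts each phase through CallGameStateTick, auto-advancing from Ready to Begin after a short delay.
; The multicast starts music through the Elebeat game instance on Ready and clears BattleBegin on End.
; Ranking refresh delegates to the world game mode, while SortRankList and the Tick rank loop are empty.
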(event `ChangeGameState_Server`
  (params (GameState :type "/Game/BluePrint/Model/Dance/EM_DanceGameState Enum" :default "NewEnumerator0"))
  (`self.ChangeGameStateMuticast` GameState)
  (switch `/Game/BluePrint/Model/Dance/EM_DanceGameState` GameState
    (:`NewEnumerator0`
      (`KismetSystemLibrary.Delay` 5.0)
      (`self.ChangeGameStateMuticast` "NewEnumerator1"))))

(event `ChangeGameStateMuticast`
  (params (GameState :type "/Game/BluePrint/Model/Dance/EM_DanceGameState Enum" :default "NewEnumerator0"))
  (bind (_nowbackgroundmusic_index _nowbackgroundmusic_musicname_cn _nowbackgroundmusic_musicname_en _nowbackgroundmusic_soundwav) (break `/Game/BluePrint/Model/Music/ST_MusicInfo` (`self.NowBackGroundMusic`)))
  (`self.GameStateTick` GameState)
  (switch `/Game/BluePrint/Model/Dance/EM_DanceGameState` GameState
    (:`NewEnumerator0`
      (bind _asbp_elebeat_gi (cast `/Game/BluePrint/AllLevel/BP_Elebeat_GI` (`GameplayStatics.GetGameInstance`)))
      (`/Game/BluePrint/AllLevel/BP_Elebeat_GI.PlayBackGroundMusic` _asbp_elebeat_gi _nowbackgroundmusic_soundwav))
    (:`NewEnumerator4`
      (set `self.BattleBegin` false))))

(event `self.ReceiveTick`
  (params (DeltaSeconds :type "Float (single-precision)"))
  (for _ (`self.Rank_PlayerList`)
    _))

(event `RefrashRankList`
  (bind _asbp_world_game_mode (cast `/Game/BluePrint/DanceGame/BP_World_GameMode` (`GameplayStatics.GetGameMode`)))
  (`/Game/BluePrint/DanceGame/BP_World_GameMode.UpdateRankingLIst` _asbp_world_game_mode))

(fn `SetUpGameInfo`
  (params (GameTime :type "Float (double-precision)"))
  (set `self.GameTime` GameTime))

(fn `SortRankList`)

(fn `UserConstructionScript`)