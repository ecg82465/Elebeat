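; BP_ScoreElement is a dance game actor that shows a Message keyword as text alongside a sphere, drifting vertically at a set Speed.
; On BeginPlay, authority only, it sets the text from the keyword enum and runs a timeline animating the sphere material's color and lighting.
; Tick moves it and turns the text toward the player camera.
; RemoveMe animates the sphere's scale by timeline, then destroys the actor.
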(event `self.ReceiveBeginPlay`
  (bind _sphere (`self.Sphere`))
  (`/Engine/EditorBlueprintResources/ActorMacros.Switch Has Authority`
    (:`Authority`
      (`|ExecutionSequence`
        (:`then_0`
          ;[1 1 1] LifeColor
          (bind (_direction _newtrack_0) (`Timeline|Timeline_0` :!via `PlayFromStart`)
            (:`Update`
              (`MeshComponent.SetVectorParameterValueOnMaterials` _sphere "Color" (`KismetMathLibrary.Conv_LinearColorToVector` _newtrack_0))
              (`MeshComponent.SetScalarParameterValueOnMaterials` _sphere "Lighting" (`.A` (break `LinearColor` _newtrack_0))))))
        (:`then_2`
          (`TextRenderComponent.K2_SetText` (`self.TextRender`) (`KismetTextLibrary.Conv_StringToText` (`|GetEnumeratorNameAsString` (`.KeyWord_11_DC3F5C5F48457831679226BCBBCE521E` (break `/Game/BluePrint/Model/Dance/Score/ST_ElementMessage` (`self.Message`)))))))))))

(event `RemoveMe`
  ;[1 1 1] Destory
  (set `self.Temp_SphereSize` (`SceneComponent.K2_GetComponentScale` (`self.Sphere`)))
  (bind (_direction _newtrack_1) (`Timeline|Timeline_1` :!via `PlayFromStart`)
    (:`Update`
      (`SceneComponent.SetWorldScale3D` (`self.Sphere`) (* (`self.Temp_SphereSize`) _newtrack_1)))
    (:`Finished`
      (`self.K2_DestroyActor`))))

(event `self.ReceiveTick`
  (params (DeltaSeconds :type "Float (single-precision)"))
  (bind _textrender (`self.TextRender`))
  (bind _returnvalue_location (`KismetMathLibrary.BreakTransform` (`self.GetTransform` (`GameplayStatics.GetPlayerCameraManager` 0))))
  (`|ExecutionSequence`
    (:`then_0`
      (set `self.Time` (+ (`self.Time`) DeltaSeconds))
      (`KismetSystemLibrary.Delay` 0.2))
    (:`then_1`
      (`self.K2_AddActorWorldOffset` (`KismetMathLibrary.MakeVector` 0.0 0.0 (* DeltaSeconds (`self.Speed`))))
      (`SceneComponent.K2_SetWorldRotation` _textrender (`KismetMathLibrary.FindLookAtRotation` (`SceneComponent.K2_GetComponentLocation` _textrender) _returnvalue_location) false false))))

(fn `UserConstructionScript`)