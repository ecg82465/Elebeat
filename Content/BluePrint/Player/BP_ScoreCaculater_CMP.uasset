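; Player rhythm-input component that spawns timed key elements and checks dance inputs against them.
; Once BeginPlayFuc enables it, Tick fires JumpTick every SpawnGateTime seconds.
; JumpTick spawns a local element through PlayerControl immediately, while a parallel delayed chain closes, briefly opens, then recloses its TikTok gate.
; CheckInput reports whether the input flag matching the first ElementList entry's keyword (W/A/S/D/Tab) is set.
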(event `JumpTick`
  (bind _playercontrol (`self.PlayerControl`))
  (`|ExecutionSequence`
    (:`then_0`
      (`/Game/BluePrint/Player/BP_PlayerControl_DJ.OpenTIckTokGate` _playercontrol false)
      (`KismetSystemLibrary.Delay` 0.3)
      (`/Game/BluePrint/Player/BP_PlayerControl_DJ.OpenTIckTokGate` _playercontrol true)
      (`KismetSystemLibrary.Delay` 0.3)
      (`/Game/BluePrint/Player/BP_PlayerControl_DJ.OpenTIckTokGate` _playercontrol false))
    (:`then_1`
      (`/Game/BluePrint/Player/BP_PlayerControl_DJ.SpawnElement_Local` _playercontrol 0.3 0.3))))

(event `self.ReceiveTick`
  (params (DeltaSeconds :type "Float (single-precision)"))
  (bind _output_get (set `self.SpawnCount` (+ (`self.SpawnCount`) DeltaSeconds)))
  (if (>= _output_get (`self.SpawnGateTime`))
    (if (`self.IsBeginPlay?`)
      (set `self.SpawnCount` 0.0)
      (`self.JumpTick`))))

(fn `BeginPlay_Fuc`
  (set `self.IsBeginPlay?` true))

(fn `CheckInput`
  (returns (Yes :type Boolean))
  (bind (_w_dance _s_dance _a_dance _d_dance _tab) (break `/Game/BluePrint/Model/Dance/ST_DanceGame_PlayerInput_Info` (`self.PlayerInputInfo`)))
  (switch `/Game/BluePrint/Model/Dance/Score/EM_Score_KeyWord` (`.KeyWord_11_DC3F5C5F48457831679226BCBBCE521E` (break `/Game/BluePrint/Model/Dance/Score/ST_ElementMessage` (`|GetArrayItem` (`self.Element_List`))))
    (:`NewEnumerator0`
      (if _w_dance
        _
        (else
          (return false))))
    (:`NewEnumerator1`
      (if _s_dance
        _
        (else
          (return false))))
    (:`NewEnumerator2`
      (if _a_dance
        _
        (else
          (return false))))
    (:`NewEnumerator3`
      (if _d_dance
        _
        (else
          (return false))))
    (:`NewEnumerator4`
      (if _tab
        _
        (else
          (return false))))
    (:`NewEnumerator6`
      (return false)))
  (return true))