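; Blueprint function library with helpers for local-player detection and camera-relative direction, plus an empty GetGameLanguage stub.
; PlayerPawnIsLocal casts to BP_Player_DJ and returns a three-state enum based on its controller type and whether the player controller ID is 0.
; CheckObjectInCameraDiraction flattens object and camera directions horizontally, using dot-product thresholds for front or back and the cross-product Z sign for left or right.
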(fn `CheckObjectInCameraDiraction`
  (params (ObjectDiraction :type "Vector Structure") (CameraDiraction :type "Vector Structure"))
  (returns (Diraction :type "/Game/BluePrint/DanceGame/BOXMap/EM_BoxDiraction Enum"))
  (bind _z (.z (`KismetMathLibrary.Cross_VectorVector` (`KismetMathLibrary.MakeVector` (.x ObjectDiraction) (.y ObjectDiraction)) (`KismetMathLibrary.MakeVector` (.x CameraDiraction) (.y CameraDiraction)))))
  (bind _returnvalue (`KismetMathLibrary.Dot_VectorVector` (`KismetMathLibrary.Normal` (`KismetMathLibrary.GreaterGreater_VectorRotator` (`KismetMathLibrary.Cross_VectorVector` ObjectDiraction (0.0 0.0 1.0)) (struct :`Yaw` 90.0))) (`KismetMathLibrary.Normal` (`KismetMathLibrary.GreaterGreater_VectorRotator` (`KismetMathLibrary.Cross_VectorVector` CameraDiraction (0.0 0.0 1.0)) (struct :`Yaw` 90.0)))))
  (if (>= _returnvalue 0.5)
    (return "NewEnumerator2")
    (elif (<= _returnvalue -0.5)
      (return "NewEnumerator3")
      (elif (>= (/ _z (`KismetMathLibrary.Abs` _z)) 0.0)
        (return "NewEnumerator0")
        (else
          (return "NewEnumerator1"))))))

(fn `GetGameLanguage`)

(fn `PlayerPawnIsLocal?`
  (params (Object :type "Pawn Object Reference"))
  (returns (IsLocal :type "/Game/BluePrint/BluePrintFunction/EM_PlayerPawnOwner Enum"))
  (bind _asbp_player_dj (cast `/Game/BluePrint/Player/BP_Player_DJ` Object)
    (:`then`
      (bind _returnvalue (`Pawn.GetController` _asbp_player_dj))
      (`/Engine/EditorBlueprintResources/StandardMacros.IsValid` _returnvalue
        (:`Is Valid`
          (bind _asplayer_controller (cast `PlayerController` _returnvalue)
            (:`then`
              (if (== (`GameplayStatics.GetPlayerControllerID` _asplayer_controller) 0)
                (return "NewEnumerator1")
                (else
                  (return "NewEnumerator0"))))
            (:`CastFailed`
              _)))
        (:`Is Not Valid`
          (return "NewEnumerator0"))))
    (:`CastFailed`
      _))
  (return "NewEnumerator2"))