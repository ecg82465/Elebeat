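; Box-grid floor for the dance game, laid out as concentric square rings walked side by side.
; The construction script previews it with numbered static meshes; BeginPlay replaces them with BP_Mapland_OneBOX actors and registers with the game mode.
; Server and multicast events recolor boxes by ID.
; The timed ring-by-ring drop is unwired, the game-state handler is empty, and key 2 calls Down(0) on every box.
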(event `self.ReceiveBeginPlay`
  (`self.Init`)
  (bind _asbp_dance_game_state (cast `/Game/BluePrint/DanceGame/BP_DanceGame_State` (`GameplayStatics.GetGameState`)))
  (add `/Game/BluePrint/DanceGame/BP_DanceGame_State.GameStateTick` _asbp_dance_game_state (delegate `CustomEvent_0`)))

(event `CustomEvent_0`
  (params (GameState :type "/Game/BluePrint/Model/Dance/EM_DanceGameState Enum" :default "NewEnumerator0"))
  (switch `/Game/BluePrint/Model/Dance/EM_DanceGameState` GameState))

(event `CustomEvent_1`
  (bind _output_get (set `self.Now_Sircle` (- (`self.Now_Sircle`) 1)))
  (for _array_element (`self.List_BoxActor`)
    (`/Game/BluePrint/DanceGame/BOXMap/BP_Mapland_OneBOX.Down` _array_element _output_get)))

(event `Key|Two`
  (params (Key :type "Key Structure"))
  (:`Pressed`
    (for _array_element (`self.List_BoxActor`)
      (`/Game/BluePrint/DanceGame/BOXMap/BP_Mapland_OneBOX.Down` _array_element 0))))

(event `ChangeBoxColor_Server`
  (params (BoxID :type Integer) (Color :type "Vector Structure"))
  (`self.ChangeBoxColor_Muticast` BoxID Color))

(event `ChangeBoxColor_Muticast`
  (params (BoxID :type Integer) (Color :type "Vector Structure"))
  (for _array_element (`self.List_BoxActor`)
    (if (== BoxID (`/Game/BluePrint/DanceGame/BOXMap/BP_Mapland_OneBOX.MyNum` _array_element))
      (`/Game/BluePrint/DanceGame/BOXMap/BP_Mapland_OneBOX.SetColor` _array_element Color))))

(fn `GluttonousSnake`
  (params (LastIndex :type Integer) (A :type "Vector Structure"))
  (returns (NewParam :type Boolean))
  (for _index (range (+ LastIndex 1))
    (bind _result (`/Engine/EditorBlueprintResources/StandardMacros.IncrementInt` (`self.Index`))
      (:`  `
        (bind _returnvalue (+ (`self.TempHead`) (* A (* (`KismetMathLibrary.Conv_IntToDouble` _index) (`self.Range`)))))
        (bind _returnvalue_2 (`AddComponent|NODE_AddStaticMeshComponent-1` :`RelativeTransform` (`KismetMathLibrary.MakeTransform` _returnvalue (struct) (`self.BOXscale`))))
        (bind _returnvalue_3 (`PrimitiveComponent.CreateDynamicMaterialInstance` _returnvalue_2 0 "/Engine/BasicShapes/BasicShapeMaterial.BasicShapeMaterial" "None"))
        (`MaterialInstanceDynamic.SetScalarParameterValue` _returnvalue_3 "Num" (`KismetMathLibrary.Conv_IntToDouble` _result))
        (`KismetArrayLibrary.Array_Add` (`self.List_Mesh_Review`) _returnvalue_2))))
  (set `self.TempHead` _returnvalue)
  (return false))

(fn `Init`
  (for _array_element (`self.List_Mesh_Review`)
    (`ActorComponent.K2_DestroyComponent` _array_element))
  (`self.SpawnAllBOX`)
  (bind _asbp_world_game_mode (cast `/Game/BluePrint/DanceGame/BP_World_GameMode` (`GameplayStatics.GetGameMode`)))
  (set `/Game/BluePrint/DanceGame/BP_World_GameMode.GamePlay_BoxLand` self _asbp_world_game_mode))

(fn `SpawnAllBOX`
  (`KismetArrayLibrary.Array_Clear` (`self.List_BoxActor`))
  (set `self.Index` 0)
  (for _index (range (`self.Circle`))
    (bind _returnvalue (* (* _index (`self.Range`)) -1.0))
    (set `self.TempHead` (`KismetMathLibrary.MakeVector` _returnvalue _returnvalue))
    (if (== _index 0)
      (`self.SpawnCircleBOX` (0.0 1.0 0.0) 0 0 _index)
      (`self.SpawnCircleBOX` (-1.0 0.0 0.0) 0 0 _index)
      (`self.SpawnCircleBOX` (0.0 -1.0 0.0) 1 0 _index)
      (else
        (bind _returnvalue_2 (* _index 2))
        (`self.SpawnCircleBOX` (1.0 0.0 0.0) (- _returnvalue_2 1) 0 _index)
        (`self.SpawnCircleBOX` (0.0 1.0 0.0) _returnvalue_2 0 _index)
        (`self.SpawnCircleBOX` (-1.0 0.0 0.0) _returnvalue_2 0 _index)
        (`self.SpawnCircleBOX` (0.0 -1.0 0.0) (+ _returnvalue_2 1) 0 _index)))))

(fn `SpawnCircleBOX`
  (params (A :type "Vector Structure") (LastIndex :type Integer) (Num :type Integer) (Circle :type Integer))
  (returns (NewParam :type Boolean))
  (for _index (range (+ LastIndex 1))
    (bind _result (`/Engine/EditorBlueprintResources/StandardMacros.IncrementInt` (`self.Index`))
      (:`  `
        (bind _returnvalue (+ (`self.TempHead`) (* A (* (`KismetMathLibrary.Conv_IntToDouble` _index) (`self.Range`)))))
        (bind _returnvalue_2 (`|SpawnActorFromClass` "/Game/BluePrint/DanceGame/BOXMap/BP_Mapland_OneBOX.BP_Mapland_OneBOX_C" (`KismetMathLibrary.MakeTransform` (+ _returnvalue (`self.K2_GetActorLocation`)) (struct) (`self.BOXscale`)) "Undefined" "OverrideRootScale" null _result Circle self null))
        (`KismetArrayLibrary.Array_Add` (`self.List_BoxActor`) _returnvalue_2))))
  (set `self.TempHead` _returnvalue)
  (return false))

(fn `UserConstructionScript`
  (`KismetArrayLibrary.Array_Clear` (`self.List_Mesh_Review`))
  (for _index (range (`self.Circle`))
    (bind _returnvalue (* (* _index (`self.Range`)) -1.0))
    (set `self.TempHead` (`KismetMathLibrary.MakeVector` _returnvalue _returnvalue))
    (if (== _index 0)
      (`self.GluttonousSnake` 0 (0.0 1.0 0.0))
      (`self.GluttonousSnake` 0 (-1.0 0.0 0.0))
      (`self.GluttonousSnake` 1 (0.0 -1.0 0.0))
      (else
        (bind _returnvalue_2 (* _index 2))
        (`self.GluttonousSnake` (- _returnvalue_2 1) (1.0 0.0 0.0))
        (`self.GluttonousSnake` _returnvalue_2 (0.0 1.0 0.0))
        (`self.GluttonousSnake` _returnvalue_2 (-1.0 0.0 0.0))
        (`self.GluttonousSnake` (+ _returnvalue_2 1) (0.0 -1.0 0.0))))))