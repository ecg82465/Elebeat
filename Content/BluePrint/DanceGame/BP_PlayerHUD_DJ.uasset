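; BP_PlayerHUD_DJ manages on-screen UI for the dance game, creating the main player HUD widget at BeginPlay.
; OpenEnter shows or removes a U_PlayerEnter prompt, creating it on first use, reusing it afterward and handing it the interaction actor.
; UpdateRankingLIst forwards ranking refresh requests to the main HUD widget.
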(event `self.ReceiveBeginPlay`
  (bind _returnvalue (`|CreateWidget` "/Game/BluePrint/UMG/PlayerInterface/U_PLayerHUD.U_PLayerHUD_C"))
  (set `self.PlayerHUD` _returnvalue)
  (`UserWidget.AddToViewport` _returnvalue 0))

(event `OpenEnter`
  (params (InteractionActor :type "Actor Object Reference") (ShowEnter :type Boolean))
  (bind _playerenter (`self.PlayerEnter`))
  (bind _playerenter_2 (`self.PlayerEnter`))
  (bind _interactionactor (`self.InteractionActor`))
  (set `self.InteractionActor` InteractionActor)
  (if ShowEnter
    (`/Engine/EditorBlueprintResources/StandardMacros.IsValid` (`self.PlayerEnter`)
      (:`Is Valid`
        _)
      (:`Is Not Valid`
        (bind _returnvalue (`|CreateWidget` "/Game/BluePrint/UMG/PlayerInterface/U_PlayerEnter.U_PlayerEnter_C" (`GameplayStatics.GetPlayerController` 0)))
        (set `self.PlayerEnter` _returnvalue)))
    (if (not (`Widget.IsVisible` _playerenter))
      (`UserWidget.AddToViewport` _playerenter 0))
    (`/Engine/EditorBlueprintResources/StandardMacros.IsValid` _interactionactor
      (:`Is Valid`
        (`/Game/BluePrint/UMG/PlayerInterface/U_PlayerEnter.GetReturnObject` _playerenter _interactionactor)))
    (else
      (`/Engine/EditorBlueprintResources/StandardMacros.IsValid` _playerenter_2
        (:`Is Valid`
          (`Widget.RemoveFromParent` _playerenter_2))))))

(event `UpdateRankingLIst`
  (`/Game/BluePrint/UMG/PlayerInterface/U_PLayerHUD.UpdateRankingList` (`self.PlayerHUD`)))

(fn `UserConstructionScript`)