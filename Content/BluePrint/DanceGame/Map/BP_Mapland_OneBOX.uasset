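; BP_Mapland_OneBOX is a single box of the DanceGame map land that sinks, rises and bobs in a wave.
; Down and Up act only when the passed value matches MyCircle, playing or reversing a timeline that lerps the actor 300 units below its start location and setting CurrentHight.
; PlayAnim runs a timeline that eases the mesh's relative Z toward a sine of BPMapLand's shared Time, phase-offset by MyNum.
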(event `self.ReceiveBeginPlay`
  (set `self.BrithLocation` (`self.K2_GetActorLocation`)))

(event `Down`
  (params (NewParam :type Integer))
  (if (== (`self.MyCircle`) NewParam)
    (set `self.CurrentHight` -300.0)
    (bind (_direction _newtrack_0) (`Timeline|EE` :!label _label)
      (:`Update`
        (`self.K2_SetActorLocation` (+ (`self.BrithLocation`) (`KismetMathLibrary.MakeVector` 0.0 0.0 (`KismetMathLibrary.Lerp` 0.0 -300.0 _newtrack_0))))))))

(event `Up`
  (params (B :type Integer))
  (if (== (`self.MyCircle`) B)
    (set `self.CurrentHight` 0.0)
    (goto _label :!via `Reverse`)))

(event `PlayAnim`
  (bind _sm_box (`self.SM_Box`))
  (bind (_relativelocation_x _relativelocation_y _relativelocation_z) (`KismetMathLibrary.BreakVector` (`SceneComponent.RelativeLocation` _sm_box)))
  (`Timeline|Timeline_0` :!via `PlayFromStart`
    (:`Update`
      (`SceneComponent.K2_SetRelativeLocation` _sm_box (`KismetMathLibrary.MakeVector` _relativelocation_x _relativelocation_y (`KismetMathLibrary.FInterpTo` _relativelocation_z (* (`KismetMathLibrary.Sin` (+ (/ (`KismetMathLibrary.Conv_IntToDouble` (`self.MyNum`)) 2.0) (`/Game/BluePrint/DanceGame/Map/BP_Mapland.Time` (`self.BP_MapLand`)))) 33.0) (`GameplayStatics.GetWorldDeltaSeconds`) 2.0)) false false))))

(fn `UserConstructionScript`)