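; BP_FlimPlane is an in-world video screen that plays a media URL entered by players.
; Overlapping its sphere makes the first local player's DJ controller show an entry UI, and SendString forwards the typed URL to that controller's UploadUrl.
; SetUpStringSetting stores the URL, whose RepNotify opens it on the MediaSound's media player.
; BeginPlay also opens the current URL and sets the widget's Chinese prompt.
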(event `self.ReceiveBeginPlay`
  (bind _asu_text (cast `/Game/BluePrint/UMG/Element/U_Text` (`WidgetComponent.GetUserWidgetObject` (`self.Widget`))))
  (`/Game/BluePrint/UMG/Element/U_Text.SetText` _asu_text "请在下方输入视频URL")
  (`MediaPlayer.OpenUrl` (`MediaSoundComponent.GetMediaPlayer` (`self.MediaSound`)) (`self.URL`)))

(event `self.Sphere.OnComponentBeginOverlap`
  (params (OverlappedComponent :type "PrimitiveComponent Object Reference") (OtherActor :type "Actor Object Reference") (OtherComp :type "PrimitiveComponent Object Reference") (OtherBodyIndex :type Integer) (bFromSweep :type Boolean) (SweepResult :type "HitResult Structure (by ref)"))
  (bind _asbp_player_dj (cast `/Game/BluePrint/Player/BP_Player_DJ` OtherActor))
  (bind _asplayer_controller (cast `PlayerController` (`Pawn.GetController` _asbp_player_dj)))
  (if (== (`GameplayStatics.GetPlayerControllerID` _asplayer_controller) 0)
    (bind _asbp_player_control_dj (cast `/Game/BluePrint/Player/BP_PlayerControl_DJ` (`GameplayStatics.GetPlayerController` 0)))
    (`/Game/BluePrint/Player/BP_PlayerControl_DJ.ShowEnterUI` _asbp_player_control_dj self true)))

(event `self.Sphere.OnComponentEndOverlap`
  (params (OverlappedComponent :type "PrimitiveComponent Object Reference") (OtherActor :type "Actor Object Reference") (OtherComp :type "PrimitiveComponent Object Reference") (OtherBodyIndex :type Integer)))

(event `/Game/BluePrint/Interface/I_ActorMessageInterface.SendString`
  (params (String :type String))
  (bind _asbp_player_control_dj (cast `/Game/BluePrint/Player/BP_PlayerControl_DJ` (`GameplayStatics.GetPlayerController` 0))
    (:`then`
      (`/Game/BluePrint/Player/BP_PlayerControl_DJ.UploadUrl` _asbp_player_control_dj String self))
    (:`CastFailed`
      (`KismetSystemLibrary.PrintString` "www"))))

(event `/Game/BluePrint/Interface/I_PlayerInteraction.SetUpString_Setting`
  (params (String :type String))
  (set `self.URL` String))

(fn `OnRep_URL`
  (`MediaPlayer.OpenUrl` (`MediaSoundComponent.GetMediaPlayer` (`self.MediaSound`)) (`self.URL`)))

(fn `UserConstructionScript`
  (bind _plane (`self.Plane`))
  (bind _returnvalue (`PrimitiveComponent.CreateDynamicMaterialInstance` _plane 0 (`PrimitiveComponent.GetMaterial` _plane 0) "None"))
  (set `self.Mat` _returnvalue))